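; Tank Blueprint that hands its barrel and turret components to their reference setters at BeginPlay and assigns the barrel mesh in the construction script.
; AimAzimuth and AimElevation axis inputs drive controller yaw and inverted pitch, scaled by frame delta time and a fixed rate.
; Alternative nodes that rotate the spring arm directly remain in the graph but are disconnected and never run.
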(event `self.ReceiveBeginPlay`
  (`self.SetBarrelReference` (`self.TankBarrel`))
  (`self.SetTurretReference` (`self.TankTurret`)))

(event `InputAxis|AimAzimuth`
  (params (AxisValue :type "Float (single-precision)"))
  (`self.AddControllerYawInput` (* AxisValue (`GameplayStatics.GetWorldDeltaSeconds`) 15.0)))

(event `InputAxis|AimElevation`
  (params (AxisValue :type "Float (single-precision)"))
  (`self.AddControllerPitchInput` (* (* AxisValue (`GameplayStatics.GetWorldDeltaSeconds`) 15.0) -1.0)))

(fn `UserConstructionScript`
  (`StaticMeshComponent.SetStaticMesh` (`self.TankBarrel`) "/Game/StaticMesh/tank_fbx_Barrel.tank_fbx_Barrel"))